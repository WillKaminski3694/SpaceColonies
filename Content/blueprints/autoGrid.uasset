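; Grid actor that procedurally builds a configurable tile grid with a highlightable selection tile.
; The construction script turns lines into quads via CreateLine, filling line and hidden selection mesh sections with dynamic M_Grid color and opacity materials.
; It also fills TileArray with tile center locations, counting one extra row and column.
; Helper functions convert between world locations and validated row/column indices, letting SetSelectedTile move or hide the highlight.
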(fn ConstructionScript
  (bind _tilesize (Variables|Constants|GettileSize))
  (bind _tilesize_2 (Variables|Constants|GettileSize))
  (bind _start (Variables|Default|Getstart))
  (bind _returnvalue (Transformation|GetWorldLocation _start))
  (bind _returnvalue_2 (/ _tilesize 2.0))
  (bind _materialinstance (Private|CreateMaterialInstance (Variables|Constants|GetlineColor) (Variables|Constants|GetlineOpacity)))
  (LocalVariables|SetLinesMaterialInstance _materialinstance)
  (bind _materialinstance_2 (Private|CreateMaterialInstance (Variables|Constants|GetselectionColor) (Variables|Constants|GetselectionOpacity)))
  (LocalVariables|SetSelectionMaterialInstance _materialinstance_2)
  (Utilities|FlowControl|Sequence
    (:then_0
      ;[1 1 1] create horizontal Line geometry
      (for _index (range 0 (Variables|Constants|GetnumRows))
        (LocalVariables|SetlineStart (* _index (Variables|Constants|GettileSize)))
        (LocalVariables|SetlineEnd (Private|GetGridWidth))
        (Private|CreateLine (Math|Vector|MakeVector (LocalVariables|GetlineStart) 0.0 0.0) (Math|Vector|MakeVector (LocalVariables|GetlineStart) (LocalVariables|GetlineEnd) 0.0) (Variables|Constants|GetlineThiccness) (LocalVariables|GetLineVertices) (LocalVariables|GetlineTriangles))))
    (:then_1
      ;[1 1 1] create vertical Line geometry
      (for _index_2 (range 0 (Variables|Constants|GetnumColumns))
        (LocalVariables|SetlineStart (* _index_2 (Variables|Constants|GettileSize)))
        (LocalVariables|SetlineEnd (Private|GetGridHeight))
        (Private|CreateLine (Math|Vector|MakeVector 0.0 (LocalVariables|GetlineStart) 0.0) (Math|Vector|MakeVector (LocalVariables|GetlineEnd) (LocalVariables|GetlineStart) 0.0) (Variables|Constants|GetlineThiccness) (LocalVariables|GetLineVertices) (LocalVariables|GetlineTriangles))))
    (:then_2
      ;[1 1 1] create line mesh
      (Class|ProceduralMeshComponent|CreateMeshSectionLinearColor (Variables|Default|GetLineMesh) 0 (LocalVariables|GetLineVertices) (LocalVariables|GetlineTriangles) 0 0 0 0 0 0 0 false false)
      (Rendering|Material|SetMaterial (Variables|Default|GetLineMesh) 0 (LocalVariables|GetLinesMaterialInstance)))
    (:then_3
      ;[1 1 1] create selection mesh
      (Private|CreateLine (Math|Vector|MakeVector 0.0 _returnvalue_2 0.0) (Math|Vector|MakeVector _tilesize_2 _returnvalue_2 0.0) _tilesize_2 (LocalVariables|Getselection%20vertices) (LocalVariables|Getselection%20Triangles))
      (Rendering|SetVisibility (Variables|Default|GetselectionMesh) false false)
      (Class|ProceduralMeshComponent|CreateMeshSectionLinearColor (Variables|Default|GetselectionMesh) 0 (LocalVariables|Getselection%20vertices) (LocalVariables|Getselection%20Triangles) 0 0 0 0 0 0 0 false false)
      (Rendering|Material|SetMaterial (Variables|Default|GetselectionMesh) 0 (LocalVariables|GetSelectionMaterialInstance)))
    (:then_4
      (LocalVariables|SethalfSize (/ (Variables|Constants|GettileSize) 2.0))
      (while (< (Variables|Default|Getinde) (* (+ (Variables|Constants|GetnumRows) 1) (+ (Variables|Constants|GetnumColumns) 1)))
        (Variables|Default|Setinde (+ (Variables|Default|Getinde) 1))
        (bind _structout (Utilities|Struct|SetmembersinautoTileStruct (Utilities|Struct|MakeautoTileStruct (LocalVariables|GetcurrentRow) (LocalVariables|GetcurrentCol) (Math|Vector|MakeVector (+ (+ (LocalVariables|GethalfSize) (* (LocalVariables|GetcurrentCol) (Variables|Constants|GettileSize))) (.x _returnvalue)) (+ (.y _returnvalue) (+ (LocalVariables|GethalfSize) (* (LocalVariables|GetcurrentRow) (Variables|Constants|GettileSize)))) (.z _returnvalue)))))
        (Utilities|Array|Add (Variables|Default|GetTileArray) _structout)
        (if (< (LocalVariables|GetcurrentCol) (Variables|Constants|GetnumColumns))
          (LocalVariables|SetcurrentCol (+ (LocalVariables|GetcurrentCol) 1))
          (else
            (LocalVariables|SetcurrentCol 0)
            (LocalVariables|SetcurrentRow (+ (LocalVariables|GetcurrentRow) 1))))))))

(fn CreateLine
  (params (Start :type Vector) (End :type Vector) (Thiccness :type Float%20%28double-precision%29) (vertices :type Array%20of%20Vectors) (triangles :type Array%20of%20Integers))
  (bind _returnvalue (Utilities|Array|Length vertices))
  (Utilities|FlowControl|Sequence
    (:then_0
      (LocalVariables|SethalfThiccness (/ Thiccness 2.0))
      (LocalVariables|SetthiccnessDirection (Math|Vector|CrossProduct (Math|Vector|Normalize (- End Start)) "0.000000,0.000000,1.000000")))
    (:then_1
      (Utilities|Array|AppendArray triangles (Utilities|Array|MakeArray (+ _returnvalue 2) (+ _returnvalue 1) (+ _returnvalue 0) (+ _returnvalue 2) (+ _returnvalue 3) (+ _returnvalue 1)))
      (Utilities|Array|AppendArray vertices (Utilities|Array|MakeArray (+ Start (* (LocalVariables|GetthiccnessDirection) (LocalVariables|GethalfThiccness))) (+ End (* (LocalVariables|GetthiccnessDirection) (LocalVariables|GethalfThiccness))) (- Start (* (LocalVariables|GetthiccnessDirection) (LocalVariables|GethalfThiccness))) (- End (* (LocalVariables|GetthiccnessDirection) (LocalVariables|GethalfThiccness))))))))

(fn GetGridWidth
  (return (* (Variables|Constants|GetnumColumns) (Variables|Constants|GettileSize))))

(fn GetGridHeight
  (return (* (Variables|Constants|GetnumRows) (Variables|Constants|GettileSize))))

(fn CreateMaterialInstance
  (params (color :type Linear%20Color%20Structure) (opacity :type Float%20%28double-precision%29))
  (bind _returnvalue (Rendering|Material|CreateDynamicMaterialInstance "/Game/blueprints/M_Grid.M_Grid" "None" "None" :!class /Script/Engine.KismetMaterialLibrary))
  (Rendering|Material|SetVectorParameterValue _returnvalue "Color" color :!class /Script/Engine.MaterialInstanceDynamic)
  (Rendering|Material|SetScalarParameterValue _returnvalue "Opacity" opacity :!class /Script/Engine.MaterialInstanceDynamic)
  (return _returnvalue))

(fn LocationtoTile
  (params (Location :type Vector))
  (bind _returnvalue (Transformation|GetActorLocation))
  (bind _returnvalue_2 (Private|GetGridHeight))
  (bind _returnvalue_3 (Transformation|GetActorLocation))
  (bind _returnvalue_4 (Private|GetGridWidth))
  (bind _numcolumns (Variables|Constants|GetnumColumns))
  (bind _numrows (Variables|Constants|GetnumRows))
  (bind _returnvalue_5 (- (.y Location) (.y _returnvalue)))
  (bind _returnvalue_6 (- (.x Location) (.x _returnvalue_3)))
  (bind _returnvalue_7 (/ _returnvalue_5 _returnvalue_4))
  (bind _returnvalue_8 (/ _returnvalue_6 _returnvalue_2))
  (bind _returnvalue_9 (* _numcolumns _returnvalue_7))
  (bind _returnvalue_10 (* _numrows _returnvalue_8))
  (bind _returnvalue_11 (Math|Float|Floor _returnvalue_9))
  (bind _returnvalue_12 (Math|Float|Floor _returnvalue_10))
  (bind _isvalid (Utilities|IsTileValid _returnvalue_12 _returnvalue_11))
  (return _isvalid _returnvalue_12 _returnvalue_11))

(fn TiletoGridLocation
  (params (row :type Integer) (column :type Integer) (center :type Boolean))
  (bind _returnvalue (Transformation|GetActorLocation))
  (bind _tilesize (Variables|Constants|GettileSize))
  (bind _returnvalue_2 (/ _tilesize 2.0))
  (bind _returnvalue_3 (select center _returnvalue_2 0.0))
  (bind _isvalid (Utilities|IsTileValid row column))
  (return _isvalid (Math|Vector2D|MakeVector2D (+ (+ (* row (Variables|Constants|GettileSize)) (.x _returnvalue)) _returnvalue_3) (+ _returnvalue_3 (+ (.y _returnvalue) (* column (Variables|Constants|GettileSize)))))))

(fn SetSelectedTile
  (params (row :type Integer) (column :type Integer))
  (bind (_isvalid _gridlocation) (CallFunction|TiletoGridLocation row column false))
  (if _isvalid
    (Rendering|SetVisibility (Variables|Default|GetselectionMesh) true false)
    (Transformation|SetWorldLocation (Variables|Default|GetselectionMesh) (Math|Vector|MakeVector (.X (Math|Vector2D|BreakVector2D _gridlocation)) (.Y (Math|Vector2D|BreakVector2D _gridlocation)) (.z (Transformation|GetActorLocation))) false false)
    (else
      (Rendering|SetVisibility (Variables|Default|GetselectionMesh) false false))))

(fn GetGridSize
  (return (Variables|Constants|GetnumRows) (Variables|Constants|GetnumColumns)))